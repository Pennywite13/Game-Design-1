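; Stealth-game enemy AI that patrols, chases and melees the player, reloading their checkpoint on a hit.
; Tick picks chase, target-point patrol or random patrol using AIMoveTo, but forces PlayerVisible true, so it always chases.
; PawnSensing handles player sightings, flashbang stuns and investigation of distraction-item noises.
; Attacks sphere-trace from the hand socket on a montage notify, with a DoOnce that resets only while Hostile.
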(event `self.ReceiveBeginPlay`
  (`self.PatrolRandom`))

(event `self.ReceiveTick`
  (params (DeltaSeconds :type "Float (single-precision)"))
  (bind _bplayervisible (`self.bPlayerVisible`))
  (set `self.bPlayerVisible` true)
  (if (`self.bCanMove`)
    (if _bplayervisible
      (`self.ChasePlayer`)
      (elif (`self.TargetPointMovement`)
        (`self.MoveToNextPatrolPoint`)
        (else
          (`self.PatrolRandom`))))
    (elif _bplayervisible
      (`self.ChasePlayer`))))

(event `self.PawnSensing.OnSeePawn`
  (params (Pawn :type "Pawn Object Reference"))
  ; Problem code is likely here
  (`|ExecutionSequence`
    (:`then_0`
      (cast `/Game/StealthGame/Gadgets/NoiseMakers/BP_Flashbang` Pawn)
      (`KismetSystemLibrary.PrintString` "THIS IS A FLASHBANG" true true (struct :`R` 1.0 :`G` 0.766374 :`A` 1.0))
      (set `self.bPlayerVisible` false)
      (set `self.bCanMove` false)
      (`KismetSystemLibrary.Delay` 8.0)
      (`KismetSystemLibrary.PrintString` "FLASHBANG OVER" true true (struct :`R` 1.0 :`G` 0.068632 :`B` 0.033291 :`A` 1.0))
      (set `self.bPlayerVisible` true)
      (set `self.bCanMove` true))
    (:`then_1`
      (cast `/Game/StealthGame/Core/Characters/PlayerCharacter/BP_ThirdPersonCharacterCustom` Pawn
        (:`then`
          (`KismetSystemLibrary.PrintString` "PLAYER SPOTTED")
          (set `self.bPlayerVisible` true))
        (:`CastFailed`
          (set `self.bPlayerVisible` false))))
    (:`then_2`
      (`KismetSystemLibrary.Delay` 1.0)
      (`KismetSystemLibrary.PrintString` "PLAYER NO LONGER SPOTTED")
      (set `self.bPlayerVisible` false))))

(event `ChasePlayer`
  (`self.UpdateWalkSpeed` 600.0)
  (set `self.bCanMove` false)
  (`|AIMoveTo` self (0.0 0.0 0.0) (`GameplayStatics.GetPlayerCharacter` 0) 50.0
    (:`OnSuccess`
      (`self.Attack`))
    (:`OnFail`
      _))
  (`KismetSystemLibrary.Delay` 3.0)
  (set `self.bCanMove` true))

(event `PatrolRandom`
  (`self.UpdateWalkSpeed` 200.0)
  (set `self.bCanMove` false)
  (`|AIMoveTo` self (`NavigationSystemV1.K2_GetRandomReachablePointInRadius` (`self.K2_GetActorLocation`) 2000.0 null null) null
    (:`OnSuccess`
      _)
    (:`OnFail`
      _))
  (`KismetSystemLibrary.Delay` 3.0)
  (set `self.bCanMove` true))

(event `MoveToNextPatrolPoint`
  (`self.UpdateWalkSpeed` 200.0)
  (set `self.bCanMove` false)
  (`|AIMoveTo` self (0.0 0.0 0.0) (`|GetArrayItem` (`self.PatrolTargetPoints`) (`self.PatrolTargetPointIndex`))
    (:`OnSuccess`
      (`KismetSystemLibrary.Delay` 3.0)
      (set `self.bCanMove` true)
      (`self.SetNextPatrolPoint`))))

(event `SetNextPatrolPoint`
  (set `self.PatrolTargetPointIndex` (mod (+ (`self.PatrolTargetPointIndex`) 1) (`KismetArrayLibrary.Array_Length` (`self.PatrolTargetPoints`)))))

(event `self.PawnSensing.OnHearNoise`
  (params (Instigator :type "Pawn Object Reference") (Location :type "Vector Structure (by ref)") (Volume :type "Float (single-precision)"))
  (bind _asbp_distraction_item_pawn (cast `/Game/StealthGame/Gadgets/NoiseMakers/BP_DistractionItemPawn` Instigator))
  (`self.UpdateWalkSpeed` 200.0)
  (set `self.bCanMove` false)
  (`|AIMoveTo` self (`/Game/StealthGame/Gadgets/NoiseMakers/BP_DistractionItemPawn.PathEndLocation` _asbp_distraction_item_pawn) null
    (:`OnSuccess`
      (`KismetSystemLibrary.Delay` 3.0)
      (set `self.bCanMove` true))))

(event `Attack`
  (bind _returnvalue (`SceneComponent.GetSocketLocation` (`self.Mesh`) "hand_r"))
  ;[0.15 0.1407 0.04319 0.5] Bonk
  (`/Engine/EditorBlueprintResources/StandardMacros.DoOnce` false :!label _label ; Only Reset Attack on miss.
    (:`Completed`
      (bind _notifyname (`|PlayMontage` (`self.Mesh`) "/Game/StealthGame/Characters/Enemies/AM_Attack_01.AM_Attack_01") ; Play the AM_Attack_01
        (:`OnCompleted`
          (if (`self.bHostile`)
            (`self.ResetAttack`) ; Resets the Do Once node.
          ))
        (:`OnNotifyBegin`
          (switch `name` _notifyname ; Pick the proper attack type(standard when there is more than one type of attack)
            (:`AttackDamage`
              (`KismetSystemLibrary.PrintString` "I'm attacking!")
              (bind (_outhits _returnvalue_2) (`KismetSystemLibrary.SphereTraceMultiForObjects` _returnvalue (+ _returnvalue (* (`self.GetActorForwardVector`) (`self.Melee Trace Distance`))) (`self.Melee Trace Radius`) (`|MakeArray` "ObjectTypeQuery3" :!type "EObjectTypeQuery Enum"))) ; Trace forward from hand socket.
              (if _returnvalue_2
                (for _array_element _outhits
                  (bind _asbp_third_person_character_custom (cast `/Game/StealthGame/Core/Characters/PlayerCharacter/BP_ThirdPersonCharacterCustom` (`.HitActor` (`GameplayStatics.BreakHitResult` _array_element))))
                  (`/Game/StealthGame/Core/Characters/PlayerCharacter/BP_ThirdPersonCharacterCustom.LoadCheckpoint` _asbp_third_person_character_custom)
                  (set `self.bHostile` false))))))))))

(event `ResetAttack`
  ;[0.15 0.1407 0.04319 0.5] Bonk
  (goto _label :!via `Reset`))

(fn `ReduceSenses`)

(fn `UpdateWalkSpeed`
  (params (NewWalkSpeed :type "Float (double-precision)"))
  (set `CharacterMovementComponent.MaxWalkSpeed` NewWalkSpeed (`self.CharacterMovement`)))

(fn `UserConstructionScript`)